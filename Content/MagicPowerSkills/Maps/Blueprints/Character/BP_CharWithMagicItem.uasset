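; Demo character for magic skill animations that spawns an attached spellbook and a reusable magic ball, and shows the current animation name on a HUD widget.
; Potion events time montages with bottle socket attachment, cap physics, liquid animation and drop impulses.
; StartAnimEvent dispatches typed effects such as AOE blow, rising balls, attraction, projectiles and a toggled shield, mostly built from BP_MagicBall actors.
; Character glow lerps emissive color on dynamic materials through a timeline.
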(event EventBeginPlay
  (Initialization|Initialize)
  (Character|PlayCharacterAnim "/Game/MagicPowerSkills/Animations/Shield/A_Shield_Start.A_Shield_Start" false)
  (Utilities|FlowControl|Delay 0.5)
  (Character|PlayCharacterAnim "/Game/MagicPowerSkills/Animations/Shield/A_Shield_Loop.A_Shield_Loop" true))

(fn ConstructionScript)

(fn SpawnMagicItem
  (params (ItemName :type String))
  (switch string ItemName
    (:Book
      (bind _returnvalue (Game|SpawnActorfromClass "/Game/MagicPowerSkills/Props/Book/Blueprints/BP_MagicBook.BP_MagicBook_C" (Transformation|GetSocketTransform (Variables|Character|GetMesh) "root" "RTS_World") "Undefined" self 0))
      (bind _output_get (Variables|MagicItem|SetBook _returnvalue))
      (Transformation|AttachActorToActor _output_get self "None" "KeepWorld" "KeepWorld" "KeepWorld" true)
      (Default|OpenBook _output_get false))))

(fn BottleTake
  (params (Bottle :type Scene%20Component%20Object%20Reference) (New%20Transform%20Location :type Vector) (New%20Transform%20Rotation :type Rotator) (SocketName :type Name))
  (Transformation|AttachComponentToComponent Bottle (Variables|Character|GetMesh) SocketName "KeepRelative" "KeepRelative" "KeepRelative" true)
  (Transformation|SetRelativeTransform Bottle (Math|Transform|MakeTransform New%20Transform%20Location New%20Transform%20Rotation "1.000000,1.000000,1.000000") false true))

(fn BottleCapOpen
  (params (Bottle :type Skeletal%20Mesh%20Component%20Object%20Reference) (Strength :type Float%20%28single-precision%29))
  (Class|SkeletalMeshComponent|SetAllBodiesBelowSimulatePhysics Bottle (Utilities|Name|MakeLiteralName "Bone_Cap") true true)
  (Physics|AddImpulse Bottle (* (Math|Vector|GetUpVector Bottle) Strength) "Bone_Cap" true)
  (Class|PrimitiveComponent|AddAngularImpulseinDegrees Bottle "0.000000,1000.000000,1000.000000" "Bone_Cap" true))

(fn BottleLiquid
  (params (Bottle :type Skeletal%20Mesh%20Component%20Object%20Reference))
  (Components|Animation|PlayAnimation Bottle "/Game/MagicPowerSkills/Props/Bottle/Animations/A_Bottle_Liquid.A_Bottle_Liquid" false))

(fn BottleDrop
  (params (Bottle :type Skeletal%20Mesh%20Component%20Object%20Reference))
  (Class|SkeletalMeshComponent|SetAllBodiesBelowSimulatePhysics Bottle (Utilities|Name|MakeLiteralName "Bone_Root") true true))

(fn PlayCharacterAnim
  (params (AnimationName :type Anim%20Sequence%20Base%20Object%20Reference) (Loop :type Boolean))
  (Class|AnimInstance|PlaySlotAnimationasDynamicMontage (Variables|Components|GetAnimBP) AnimationName "DefaultSlot" 0.25 0.4 1.0 (select Loop 99999 1) -1.0 0.0)
  (bind _output_get (LocalVariables|SetAnimNameArray (Utilities|String|GetCharacterArrayfromString (Utilities|GetDisplayName AnimationName))))
  (Utilities|Array|RemoveIndex _output_get)
  (Utilities|Array|RemoveIndex _output_get)
  (Default|SetAnimNameText (Variables|Hud|GetHudAnimName) (Utilities|String|JoinStringArray (LocalVariables|GetAnimNameArray) "")))

(fn BottleRestore
  (params (Bottle :type Skeletal%20Mesh%20Component%20Object%20Reference))
  (Physics|SetSimulatePhysics Bottle false)
  (Transformation|AttachComponentToComponent Bottle (Variables|Character|GetMesh) "pelvis" "KeepRelative" "KeepRelative" "KeepRelative" true)
  (Transformation|SetRelativeTransform Bottle (select (== Bottle (Variables|Default|GetBottleLeft)) (Math|Transform|MakeTransform "11.021629,-1.310582,-16.054917" "-90.000000,7.125016,52.874983" "0, 0, 0") (Math|Transform|MakeTransform "11.021629,-1.310582,16.283847" "-90.000000,0.000000,60.000000" "0, 0, 0")) false true)
  (Components|Animation|PlayAnimation Bottle "/Game/MagicPowerSkills/Props/Bottle/Animations/A_Bottle_Liquid_Restore.A_Bottle_Liquid_Restore" false))

(event Custom|CloseBook
  (Utilities|IsValid (Variables|MagicItem|GetBook)
    (:Is%20Valid
      (Default|OpenBook (Variables|MagicItem|GetBook) false)
      (Variables|/Game/MagicPowerSkills/Maps/Blueprints/Character/AnimBP_Demo.AnimBP_Demo_C|SetIsUseBook (Variables|Components|GetAnimBP) false))))

(event Custom|OpenBook
  (Utilities|IsValid (Variables|MagicItem|GetBook)
    (:Is%20Valid
      (Default|OpenBook (Variables|MagicItem|GetBook) true)
      (Variables|/Game/MagicPowerSkills/Maps/Blueprints/Character/AnimBP_Demo.AnimBP_Demo_C|SetIsUseBook (Variables|Components|GetAnimBP) true))))

(event Custom|PotionDrinkLeft
  (Bottle|BottleRestore (Variables|Default|GetBottleLeft))
  (Character|PlayCharacterAnim "/Game/MagicPowerSkills/Animations/Potion/A_Potion_01.A_Potion_01" false)
  (Utilities|FlowControl|Delay 0.33)
  (Bottle|BottleTake (Variables|Default|GetBottleLeft) "7.292901,-4.144589,1.967469" "-7.374801,-88.887007,164.626365" "hand_l")
  (Utilities|FlowControl|Delay 0.32)
  (Bottle|BottleCapOpen (Variables|Default|GetBottleLeft) 2e+02)
  (Utilities|FlowControl|Delay 0.53)
  (Bottle|BottleLiquid (Variables|Default|GetBottleLeft))
  (Utilities|FlowControl|Delay 0.65)
  (Bottle|BottleDrop (Variables|Default|GetBottleLeft)))

(event Custom|PotionBlow
  (bind _bottleleft (Variables|Default|GetBottleLeft))
  (Bottle|BottleRestore (Variables|Default|GetBottleLeft))
  (Character|PlayCharacterAnim "/Game/MagicPowerSkills/Animations/Potion/A_Potion_Blow.A_Potion_Blow" false)
  (Utilities|FlowControl|Delay 0.31)
  (Bottle|BottleTake (Variables|Default|GetBottleLeft) "7.292901,-4.144589,1.967469" "-7.374801,-88.887007,164.626365" "hand_l")
  (Bottle|BottleLiquid _bottleleft)
  (Utilities|FlowControl|Delay 0.58)
  (Bottle|BottleDrop _bottleleft)
  (Physics|AddImpulse _bottleleft "0.000000,400.000000,-600.000000" "Bone_Root" true))

(event Custom|PotionDrinkRight
  (Bottle|BottleRestore (Variables|Default|GetBottleRight))
  (Character|PlayCharacterAnim "/Game/MagicPowerSkills/Animations/Potion/A_Potion_02.A_Potion_02" false)
  (Utilities|FlowControl|Delay 0.4)
  (Bottle|BottleTake (Variables|Default|GetBottleRight) "-8.637296,3.699927,-2.308339" "0, 0, 0" "hand_r")
  (Utilities|FlowControl|Delay 0.15)
  (Bottle|BottleCapOpen (Variables|Default|GetBottleRight) 1e+02)
  (Utilities|FlowControl|Delay 0.4)
  (Bottle|BottleLiquid (Variables|Default|GetBottleRight))
  (Utilities|FlowControl|Delay 0.85)
  (Bottle|BottleDrop (Variables|Default|GetBottleRight)))

(event Custom|PotionThtrow
  (bind _bottleright (Variables|Default|GetBottleRight))
  (Bottle|BottleRestore (Variables|Default|GetBottleRight))
  (Character|PlayCharacterAnim "/Game/MagicPowerSkills/Animations/Potion/A_Potion_Throw.A_Potion_Throw" false)
  (Utilities|FlowControl|Delay 0.4)
  (Bottle|BottleTake (Variables|Default|GetBottleRight) "7.292901,-4.144589,1.967469" "-7.374801,-88.887007,164.626365" "hand_l")
  (Utilities|FlowControl|Delay 0.2)
  (Bottle|BottleDrop _bottleright)
  (Physics|AddImpulse _bottleright "0.000000,100.000000,20.000000" "Bone_Root" true))

(event Custom|StartAnimEvent
  (params (Type :type E_AnimNotifyType%20Enum :default "NewEnumerator0") (BoneLocName :type Name) (Time :type Float%20%28double-precision%29) (GlowColor :type Linear%20Color%20Structure) (LocalLocation :type Vector))
  (switch Utilities|FlowControl|Switch|SwitchonE_AnimNotifyType Type
    (:NewEnumerator0
      (|AOEBlow BoneLocName LocalLocation))
    (:NewEnumerator1
      (|BallsUp))
    (:NewEnumerator2
      (CallFunction|SetCharEm Time GlowColor))
    (:NewEnumerator4
      (|Attraction BoneLocName Time LocalLocation))
    (:NewEnumerator5
      (|Direct Time BoneLocName LocalLocation))
    (:NewEnumerator7
      (|Up Time BoneLocName LocalLocation))
    (:NewEnumerator8
      (|Shield))))

(event Custom|AOE-Blow
  (Transformation|SetActorScale3D (Variables|Components|GetMagicBall) "0, 0, 0")
  (Rendering|Material|SetScalarParameterValue (Variables|/Game/MagicPowerSkills/Maps/Blueprints/MagicBall/BP_MagicBall.BP_MagicBall_C|GetMaterial (Variables|Components|GetMagicBall)) "Opacity" 1.0 :!class /Script/Engine.MaterialInstanceDynamic)
  (Components|Activation|SetActive (Variables|Default|GetWaveEffect) true false)
  (Rendering|SetActorHiddenInGame (Variables|Components|GetMagicBall) false)
  (Components|Activation|SetActive (Variables|/Game/MagicPowerSkills/Maps/Blueprints/MagicBall/BP_MagicBall.BP_MagicBall_C|GetEffectTrail (Variables|Components|GetMagicBall)) true false)
  (Default|SetScale (Variables|Components|GetMagicBall) 0.3 "25.000000,25.000000,25.000000")
  (Default|SetOpacity (Variables|Components|GetMagicBall) 0.3 0.5)
  (Default|SetScale (Variables|Components|GetMagicBall) 0.3 "30.000000,30.000000,30.000000")
  (Default|SetOpacity (Variables|Components|GetMagicBall) 0.3 0.0)
  (Utilities|FlowControl|Delay 0.2)
  (Components|Activation|SetActive (Variables|/Game/MagicPowerSkills/Maps/Blueprints/MagicBall/BP_MagicBall.BP_MagicBall_C|GetEffectTrail (Variables|Components|GetMagicBall)) false false))

(event Custom|SetTransformEffects
  (params (TranformWave :type Transform) (TransformBall :type Transform))
  (Transformation|SetWorldTransform (Variables|Default|GetWaveEffect) TranformWave false false)
  (Transformation|SetActorTransform (Variables|Components|GetMagicBall) TransformBall))

(event Custom|SetCharEm
  (params (Time :type Float%20%28double-precision%29) (ColorTarget :type Linear%20Color%20Structure))
  (Components|Timeline|SetPlayRate (Variables|Default|GetTM_Color) (/ 1.0 Time))
  (Variables|Material|SetColorTarget ColorTarget)
  (bind _returnvalue (Rendering|Material|GetVectorParameterValue (Variables|Material|GetCharMaterial01) "EmisiveColor" :!class /Script/Engine.MaterialInstanceDynamic))
  (Variables|Material|SetColorCurrent _returnvalue)
  (bind _alpha (Timeline|TM_Color PlayFromStart)
    (:Update
      (Rendering|Material|SetVectorParameterValue (Variables|Material|GetCharMaterial01) "EmisiveColor" (Math|Color|Lerp(LinearColor) (Variables|Material|GetColorCurrent) (Variables|Material|GetColorTarget) _alpha) :!class /Script/Engine.MaterialInstanceDynamic))))