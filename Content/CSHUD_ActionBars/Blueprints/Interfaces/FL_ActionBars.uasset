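; Blueprint function library that gives other code quick access to the action bars HUD and its ACActionBars manager component.
; Lookups start from player zero, a given player controller, a generic controller or a player index, then cast that controller's HUD to CSHUD_ActionBars.
; The manager getters print an error on a failed cast, using leftover ShooterHUD names, while the HUD getter fails silently.
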(fn GetShooterHudManager
  (bind _ascshud_action_bars (Utilities|Casting|CastToCSHUD_ActionBars (HUD|GetHUD (Game|GetPlayerController 0)))
    (:then
      (return (Variables|/Game/CSHUD_ActionBars/Blueprints/CSHUD_ActionBars.CSHUD_ActionBars_C|GetAC_ActionBars _ascshud_action_bars)))
    (:CastFailed
      (Development|PrintString 0 "FL_ShooterHUD: Cast to HUD_CompShooter failed!" true true "(R=1.000000,G=0.230857,B=0.000000,A=1.000000)" 1e+01))))

(fn GetShooterHudManagerfromPlayer
  (params (PlayerController :type Player%20Controller%20Object%20Reference))
  (bind _ascshud_action_bars (Utilities|Casting|CastToCSHUD_ActionBars (HUD|GetHUD PlayerController))
    (:then
      (return (Variables|/Game/CSHUD_ActionBars/Blueprints/CSHUD_ActionBars.CSHUD_ActionBars_C|GetAC_ActionBars _ascshud_action_bars)))
    (:CastFailed
      (Development|PrintString 0 "FL_ShooterHUD: Cast to HUD_CompShooter failed!" true true "(R=1.000000,G=0.230857,B=0.000000,A=1.000000)" 1e+01))))

(fn GetShooterHudManagerfromController
  (params (Controller :type Controller%20Object%20Reference))
  (bind _asplayer_controller (Utilities|Casting|CastToPlayerController Controller)
    (:then
      (bind _ascshud_action_bars (Utilities|Casting|CastToCSHUD_ActionBars (HUD|GetHUD _asplayer_controller))
        (:then
          (return (Variables|/Game/CSHUD_ActionBars/Blueprints/CSHUD_ActionBars.CSHUD_ActionBars_C|GetAC_ActionBars _ascshud_action_bars)))
        (:CastFailed
          (Development|PrintString 0 "FL_ShooterHUD: Cast to HUD_CompShooter failed!" true true "(R=1.000000,G=0.230857,B=0.000000,A=1.000000)" 1e+01))))
    (:CastFailed
      (Development|PrintString 0 "FL_ShooterHUD: Cast to PlayerController Instance failed!" true true "(R=1.000000,G=0.230857,B=0.000000,A=1.000000)" 1e+01))))

(fn GetShooterHud
  (params (PlayerIndex :type Integer))
  (bind _ascshud_action_bars (Utilities|Casting|CastToCSHUD_ActionBars (HUD|GetHUD (Game|GetPlayerController 0 PlayerIndex))))
  (return _ascshud_action_bars))