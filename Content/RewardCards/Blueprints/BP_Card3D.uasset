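; BP_Card3D is a 3D reward card that flips open to reveal a random reward from its owning BP_CardsDeck.
; Opening draws from the deck's level pool, optionally removes repeats, updates the mesh and UW_Card widget, and notifies the deck.
; Timelines drive the flip, optional randomly offset float and hover slide, with float and slide sharing one location vector applied on Tick.
; Hover also adjusts glow and aura through dynamic materials.
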(event Custom|GetRandomInfoForCard
  ;[1 1 1] Get random info for card when user clicked on card
  (bind _asbp_cards_deck (Utilities|Casting|CastToBP_CardsDeck (Components|GetOwner)))
  (bind _rewardcard (Default|GetRandomRewardCard (Variables|Default|GetAC_RandomCard) (Variables|/Game/RewardCards/Blueprints/BP_CardsDeck.BP_CardsDeck_C|GetReward%20Cards%20for%20Level _asbp_cards_deck)))
  (bind _output_get (Variables|Default|SetCardInfo _rewardcard))
  (CallFunction|UpdateCardRewardSide _rewardcard)
  (if (Variables|/Game/RewardCards/Blueprints/BP_CardsDeck.BP_CardsDeck_C|GetNoRepeats _asbp_cards_deck)
    (Utilities|Array|RemoveItem (Variables|/Game/RewardCards/Blueprints/BP_CardsDeck.BP_CardsDeck_C|GetReward%20Cards%20for%20Level _asbp_cards_deck) _output_get)))

(event Custom|UpdateHoverCardState
  (params (E_CardState :type E_HoverCardState%20Enum :default "NewEnumerator1"))
  ;[0.06771 0.06771 0.06771] Update Card State
  (bind _output_get (Variables|Default|SetCardHoverState E_CardState))
  (switch Utilities|FlowControl|Switch|SwitchonE_HoverCardState _output_get
    (:NewEnumerator1
      ;;[1 1 1] UnHovered
      (CallFunction|UnHoveredStyle 33.0 0.1)
      (CallFunction|MoveCard false))
    (:NewEnumerator0
      ;;[1 1 1] Hovered Style
      (CallFunction|HoverStyle 1e+02 1.0)
      (CallFunction|MoveCard true))))

(event Custom|UpdateCardState
  (params (CardState :type E_CardState%20Enum :default "NewEnumerator0"))
  ;[0.06771 0.06771 0.06771] Update Card State
  (Variables|Default|SetCardState CardState))

(event Custom|RotateCard
  ;[0.06771 0.06771 0.06771] Rotate card
  (if (Variables|Default|GetCanRotate)
    (Variables|Default|SetCanRotate false)
    (Components|Timeline|SetPlayRate (Variables|Default|GetRotatingCard) 1.0)
    (bind _newtrack_0 (Timeline|RotatingCard PlayFromStart)
      (:Update
        (Transformation|SetRelativeRotation (Variables|Default|GetRotatingScene) (Math|Rotator|MakeRotator 0.0 0.0 (Math|Float|Lerp 0.0 -1.8e+02 _newtrack_0)) false false)))))

(event Custom|UpdateCardRewardSide
  (params (CardInfo :type S%20Card%20Info%20Structure))
  (bind (_rewardbg _rewardicon _cardmesh3d) (Utilities|Struct|BreakS_CardInfo CardInfo))
  ;[0.06771 0.06771 0.06771] Update RewardSide of the card
  (bind _asuw_card (Utilities|Casting|CastToUW_Card (UserInterface|GetWidget (Variables|Default|GetWidgetRewardSide))))
  (Default|UpdateImage _asuw_card _rewardbg _rewardicon)
  (Components|StaticMesh|SetStaticMesh (Variables|Default|GetSM_CardMesh) _cardmesh3d))

(event Custom|OnCursorHovered_Event
  ;[0.06771 0.06771 0.06771] On mouse hovered
  (CallFunction|UpdateHoverCardState "NewEnumerator0"))

(event Custom|OnCardOpen_Event
  ;[0.06771 0.06771 0.06771] On Card Open
  (if (Utilities|Enum|Equal(Enum) (Variables|Default|GetCardState) "NewEnumerator0")
    (if (Utilities|Array|IsNotEmpty (Variables|/Game/RewardCards/Blueprints/BP_CardsDeck.BP_CardsDeck_C|GetReward%20Cards%20for%20Level (.AsBP%20Cards%20Deck (Utilities|Casting|CastToBP_CardsDeck (Components|GetOwner)))))
      (CallFunction|GetRandomInfoforCard)
      (CallFunction|RotateCard)
      (CallFunction|UpdateCardState "NewEnumerator1")
      ;[1 0.5841 0] REWARD RECEIVED
      (bind _asbp_cards_deck (Utilities|Casting|CastToBP_CardsDeck (Components|GetOwner)))
      (Default|CallOnRewardReceived _asbp_cards_deck (Utilities|Struct|BreakS_CardInfo (Variables|Default|GetCardInfo)))
      (else
        (Development|PrintString "Cant open , no unique cards left, (Set bool NoRepeat to False) in BP_CardSet" true true "(R=1.000000,G=0.000000,B=0.006409,A=1.000000)")))))

(event Custom|CreateDynamicMaterials
  (bind _sm_cardmesh (Variables|Default|GetSM_CardMesh))
  ;[0.06771 0.06771 0.06771] Create dynamic materials
  (bind _returnvalue (Rendering|Material|CreateDynamicMaterialInstance _sm_cardmesh 3 0 "None" :!class /Script/Engine.PrimitiveComponent))
  (Variables|Default|SetDynMat3 _returnvalue)
  (bind _returnvalue_2 (Rendering|Material|CreateDynamicMaterialInstance _sm_cardmesh 5 0 "None" :!class /Script/Engine.PrimitiveComponent))
  (Variables|Default|SetDynMat4 _returnvalue_2)
  (bind _returnvalue_3 (Rendering|Material|CreateDynamicMaterialInstance (Variables|Default|GetSM_Aura) 0 0 "None" :!class /Script/Engine.PrimitiveComponent))
  (Variables|Default|SetDynMatAura _returnvalue_3))

(event Custom|MoveCard
  (params (ToFront :type Boolean))
  (bind _rotatingscene (Variables|Default|GetRotatingScene))
  (bind _relativelocation (Variables|/Script/Engine.SceneComponent|GetRelativeLocation _rotatingscene))
  ;[0.06771 0.06771 0.06771] Update Card State
  ;;[1 1 1] Card move forward animation
  (Components|Timeline|SetPlayRate (Variables|Default|GetCardMoveForw) 4.0)
  (if ToFront
    (bind _newtrack_0 (Timeline|CardMoveForw PlayFromStart)
      (:Update
        (Variables|Default|SetAnimationRelLoc (Math|Vector|MakeVector (.X (Math|Vector|BreakVector (Math|Vector|Lerp(Vector) (.location (Variables|Default|GetSavedCardStartTransform)) (Math|Vector|MakeVector (Variables|CardAnimation|GetForwardMoveOnHover) (.y _relativelocation) (.z _relativelocation)) _newtrack_0))) (.Y (Math|Vector|BreakVector (Variables|Default|GetAnimationRelLoc))) (.Z (Math|Vector|BreakVector (Variables|Default|GetAnimationRelLoc)))))))
    (else
      (Timeline|CardMoveForw ReverseFromEnd))))

(event Custom|UpdateCardBackSide
  (params (CardInfo :type S%20Card%20Info%20Structure))
  (bind (_backsidebg _backsideicon _cardmesh3d) (Utilities|Struct|BreakS_CardInfo CardInfo))
  ;[0.06771 0.06771 0.06771] Update Backside of the card
  (bind _asuw_card (Utilities|Casting|CastToUW_Card (UserInterface|GetWidget (Variables|Default|GetWidgetBackSide))))
  (Default|UpdateImage _asuw_card _backsidebg _backsideicon)
  (Components|StaticMesh|SetStaticMesh (Variables|Default|GetSM_CardMesh) _cardmesh3d))

(event EventTick
  (params (DeltaSeconds :type Float%20%28single-precision%29))
  ;[1 1 1] Update Relative location
  (Transformation|SetRelativeLocation (Variables|Default|GetRotatingScene) (Variables|Default|GetAnimationRelLoc) false false))

(event EventBeginPlay
  (EventDispatchers|BindEventtoOnCardOpened (EventDispatchers|CreateEvent :!event Custom|OnCardOpen_Event))
  (EventDispatchers|BindEventtoOnCursorHovered (EventDispatchers|CreateEvent :!event Custom|OnCursorHovered_Event))
  (CallFunction|CreateDynamicMaterials)
  (Variables|Default|SetSavedCardStartTransform (Transformation|GetRelativeTransform (Variables|Default|GetRotatingScene)) :!pinned true) ; Save default transform
  ;[1 1 1] Floating
  (if (Variables|CardAnimation|GetCardFloating)
    (Utilities|FlowControl|Delay (Math|Random|RandomFloatinRange 0.0 1.0))
    (Components|Timeline|SetPlayRate (Variables|Default|GetFloating) 0.5)
    (bind _newtrack_0 (Timeline|Floating PlayFromStart)
      (:Update
        (Variables|Default|SetAnimationRelLoc (Math|Vector|MakeVector (.x (Variables|Default|GetAnimationRelLoc)) (.y (Variables|Default|GetAnimationRelLoc)) (Math|Float|Lerp 0.0 (Variables|CardAnimation|GetFloatingMove) _newtrack_0)))))))

(fn ConstructionScript
  (bind (_cardinfo _foundcard) (CallFunction|MFGetCardInfobyID (Variables|Default|GetCardID)))
  (if _foundcard
    (bind _output_get (Variables|Default|SetCardInfo _cardinfo))
    (CallFunction|UpdateCardBackSide _output_get)
    (CallFunction|UpdateCardRewardSide _output_get)))

(fn HoverStyle
  (params (EmissivePower :type Float%20%28single-precision%29) (AuraIntensity :type Float%20%28single-precision%29))
  (Rendering|Material|SetScalarParameterValue (Variables|Default|GetDynMat3) "EmissivePower" EmissivePower :!class /Script/Engine.MaterialInstanceDynamic)
  (Rendering|Material|SetScalarParameterValue (Variables|Default|GetDynMatAura) "MainMultiply" AuraIntensity :!class /Script/Engine.MaterialInstanceDynamic)
  (Development|SetHiddeninGame (Variables|Default|GetSM_Cylinder) false false))

(fn UnHoveredStyle
  (params (EmissivePower :type Float%20%28single-precision%29) (AuraIntensity :type Float%20%28single-precision%29))
  (Rendering|Material|SetScalarParameterValue (Variables|Default|GetDynMat3) "EmissivePower" EmissivePower :!class /Script/Engine.MaterialInstanceDynamic)
  (Rendering|Material|SetScalarParameterValue (Variables|Default|GetDynMatAura) "MainMultiply" AuraIntensity :!class /Script/Engine.MaterialInstanceDynamic)
  (Development|SetHiddeninGame (Variables|Default|GetSM_Cylinder) true false))