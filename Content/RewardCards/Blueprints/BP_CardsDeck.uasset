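; BP_CardsDeck is a reward card deck actor that spawns a centered grid of BP_Card3D cards for the current reward level.
; At BeginPlay it looks up that level's reward cards, builds the grid and binds a reward-received event, currently a debug-print placeholder for reward logic.
; Next/previous events move a clamped selection index to hover cards for controller input.
; Setting changes destroy and respawn all cards.
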(event Custom|OnRewardRecieved_Event
  (params (RewardID :type Integer))
  ;[1 0.4171 0] REWARD ITEM RECEIVED (Implement logic for rewards here)
  (Development|PrintString (Utilities|String|Append (Utilities|GetDisplayName self) ": " "REWARD RECEIVED WITH ID= " (Utilities|String|ToString(Integer) RewardID)) true false "(R=1.000000,G=0.420983,B=0.000000,A=1.000000)" 1e+01))

(event Custom|SpawnCards
  ;[0.06771 0.06771 0.06771] Spawn cards
  (bind (_rewardcardsforlevel _found) (CallFunction|MFGetRewardCardforLevel (Variables|Default|GetRewardForLevel)))
  (if _found
    (Variables|Default|SetReward%20Cards%20for%20Level _rewardcardsforlevel)
    (bind _itempos1 (CallFunction|PlaceCardsinGrid (Variables|Default|GetRowsNumber) (Variables|Default|GetCardsInRow) (Variables|Default|GetDistanceBetweenCards)))
    (for _array_element _itempos1
      (bind _returnvalue (Game|SpawnActorfromClass "/Game/RewardCards/Blueprints/BP_Card3D.BP_Card3D_C" (Math|Transform|MakeTransform (Math|Vector|MakeVector (.x (Transformation|GetActorLocation)) (.Y (Math|Vector|BreakVector _array_element)) (.Z (Math|Vector|BreakVector _array_element))) "0, 0, 0" "1.000000,1.000000,1.000000") "Undefined" self (Variables|Default|GetFloatingCards) 0 0)) ; Spawn Default Cards
      (Utilities|Array|Add (Variables|Default|GetSpawnedCards) _returnvalue)
      (Variables|Default|SetControllerSelectedCard 0)
      (Variables|Default|SetMaxCardIndex (- (* (Variables|Default|GetRowsNumber) (Variables|Default|GetCardsInRow)) 1)))))

(event Custom|RespawnCards
  ;[0.06771 0.06771 0.06771] Spawn cards
  (for _array_element (Variables|Default|GetSpawnedCards)
    (Actor|DestroyActor _array_element))
  (Utilities|Array|Clear (Variables|Default|GetSpawnedCards))
  (Utilities|Array|Clear (Variables|Default|GetOpenedCardIDs))
  (CallFunction|SpawnCards)
  (Class|WidgetBlueprintLibrary|SetFocustoGameViewport))

(event EventBeginPlay
  ;[0.06771 0.06771 0.06771] Begin play
  (CallFunction|SpawnCards)
  (EventDispatchers|BindEventtoOnRewardReceived (delegate Custom|OnRewardRecieved_Event)))

(event EventSelectPrevCard
  (bind _spawnedcards (Variables|Default|GetSpawnedCards))
  ;[0.06771 0.06771 0.06771] Controller select next/prev card
  (Utilities|UnHoverCard (Variables|Default|GetControllerSelectedCard))
  (Variables|Default|SetControllerSelectedCard (Math|Integer|Clamp(Integer) (+ (Variables|Default|GetControllerSelectedCard) -1) 0 (Variables|Default|GetMaxCardIndex)))
  (if (Utilities|Array|IsValidIndex _spawnedcards (Variables|Default|GetControllerSelectedCard))
    (Utilities|IsValid (Utilities|Array|Get(acopy) _spawnedcards (Variables|Default|GetControllerSelectedCard))
      (:Is%20Valid
        (Default|CallOnCursorHovered (Utilities|Array|Get(acopy) _spawnedcards (Variables|Default|GetControllerSelectedCard)))))))

(event EventSelectNextCard
  (bind _spawnedcards (Variables|Default|GetSpawnedCards))
  ;[0.06771 0.06771 0.06771] Controller select next/prev card
  (Utilities|UnHoverCard (Variables|Default|GetControllerSelectedCard))
  (Variables|Default|SetControllerSelectedCard (Math|Integer|Clamp(Integer) (+ (Variables|Default|GetControllerSelectedCard) 1) 0 (Variables|Default|GetMaxCardIndex)))
  (if (Utilities|Array|IsValidIndex _spawnedcards (Variables|Default|GetControllerSelectedCard))
    (Utilities|IsValid (Utilities|Array|Get(acopy) _spawnedcards (Variables|Default|GetControllerSelectedCard))
      (:Is%20Valid
        (Default|CallOnCursorHovered (Utilities|Array|Get(acopy) _spawnedcards (Variables|Default|GetControllerSelectedCard)))))))

(event EventSetRepeatsinDeck
  (params (NoRepeats :type Boolean))
  ;[0.06771 0.06771 0.06771] Deck Settings
  (Variables|Default|SetNoRepeats NoRepeats)
  (CallFunction|RespawnCards))

(event EventSetCardsinRow
  (params (CardsInRow :type Integer))
  ;[0.06771 0.06771 0.06771] Deck Settings
  (Variables|Default|SetCardsInRow CardsInRow)
  (CallFunction|RespawnCards))

(event EventSetNumberOfRows
  (params (RowsNumber :type Integer))
  ;[0.06771 0.06771 0.06771] Deck Settings
  (Variables|Default|SetRowsNumber RowsNumber)
  (CallFunction|RespawnCards))

(event EventSetNumberOfAttempts
  (params (NumOfAttempts :type Integer))
  ;[0.06771 0.06771 0.06771] Deck Settings
  (Variables|Default|SetNumberOfAttempts NumOfAttempts)
  (CallFunction|RespawnCards))

(event EventSetRewardLevel
  (params (RewardLevel :type Integer))
  ;[0.06771 0.06771 0.06771] Deck Settings
  (bind _output_get (Variables|Default|SetRewardForLevel RewardLevel))
  (Development|PrintString (Utilities|String|Append "Reward Level changed to: " (Utilities|String|ToString(Integer) _output_get)) true false)
  (CallFunction|RespawnCards))

(event EventSetFloatingCards
  (params (FloatingCards :type Boolean))
  ;[0.06771 0.06771 0.06771] Deck Settings
  (Variables|Default|SetFloatingCards FloatingCards)
  (CallFunction|RespawnCards))

(fn ConstructionScript
  (Variables|Info|SetOverallCardsCount (* (Variables|Default|GetCardsInRow) (Variables|Default|GetRowsNumber))))

(fn GetSelectedCard
  (bind _controllerselectedcard (Variables|Default|GetControllerSelectedCard))
  (bind _spawnedcards (Variables|Default|GetSpawnedCards))
  (if (Utilities|Array|IsValidIndex _spawnedcards _controllerselectedcard)
    (return (Utilities|Array|Get(acopy) _spawnedcards _controllerselectedcard) true)
    (else
      (return 0 false))))

(fn PlaceCardsinGrid
  (params (NumRows :type Integer) (NumCols :type Integer) (GridSpacing :type Float%20%28double-precision%29))
  (Utilities|FlowControl|Sequence
    (:then_0
      (LocalVariables|SetTotalWidth (* (- NumCols 1) GridSpacing))
      (LocalVariables|SetTotalHeight (* (- NumRows 1) GridSpacing))
      (LocalVariables|SetTableLoc (- (Transformation|GetActorLocation) (Math|Vector|MakeVector 0.0 (* (LocalVariables|GetTotalWidth) 0.5) (* (LocalVariables|GetTotalHeight) 0.5))))
      (LocalVariables|SetTotalItems (* NumRows NumCols))
      (bind _index (Utilities|FlowControl|ForLoopwithBreak 0 (- NumRows 1))
        (:LoopBody
          (LocalVariables|SetRowIndex _index)
          (bind _index_2 (Utilities|FlowControl|ForLoopwithBreak 0 (- NumCols 1) :!label _label)
            (:LoopBody
              (LocalVariables|SetColIndex _index_2)
              (bind _output_get (LocalVariables|SetItemIndex (+ (* (LocalVariables|GetRowIndex) NumCols) (LocalVariables|GetColIndex))))
              (if (>= _output_get (LocalVariables|GetTotalItems))
                (goto _label Break)
                (else
                  (Utilities|Array|Add (LocalVariables|GetItemPos) (+ (LocalVariables|GetTableLoc) (Math|Vector|MakeVector 0.0 (* (LocalVariables|GetColIndex) GridSpacing) (* (LocalVariables|GetRowIndex) GridSpacing)))))))))))
    (:then_1
      (return (LocalVariables|GetItemPos)))))