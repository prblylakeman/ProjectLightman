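; Blueprint interface for the action manager of a shooter HUD with health, armor, weapon and action-slot bars.
; It declares calls to display the HUD, add or remove styled bars, update or reduce health, armor and ammo, and query their current values.
; Further calls manage ammo icons and keyed action slots, including a slot impact call.
; All functions are empty declarations, leaving the behavior to implementers.
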(fn DisplayShooterHUD
  (params (State :type E_DisplayStates%20Enum) (ZOrder :type Integer)))

(fn AddHealthBar
  (params (ProgressBar_Color :type Linear%20Color%20Structure) (Progress_Color :type Linear%20Color%20Structure) (Text_Color :type Linear%20Color%20Structure) (Frame_Color :type Linear%20Color%20Structure) (Damage_Color :type Linear%20Color%20Structure) (Health_Color :type Linear%20Color%20Structure) (Icon :type User%20Widget%20Class%20Reference) (IsMaxHealthSensitive :type Boolean)))

(fn RemoveHealthBar)

(fn UpdateHealth
  (params (Value :type Integer) (UpdateType :type E_UpdateTypes%20Enum)))

(fn UpdateMaxHealth
  (params (Max_Health_Value :type Integer)))

(fn GetCurrentHealth
  (return 0))

(fn GetCurrentMaxHealth
  (return 0))

(fn RemoveHealth
  (params (DamageValue :type Integer)))

(fn AddArmorBar
  (params (ProgressBar_Color :type Linear%20Color%20Structure) (Progress_Color :type Linear%20Color%20Structure) (Text_Color :type Linear%20Color%20Structure) (Frame_Color :type Linear%20Color%20Structure) (Damage_Color :type Linear%20Color%20Structure) (Armor_Color :type Linear%20Color%20Structure) (Armor_Icon :type User%20Widget%20Class%20Reference) (MaxArmorSensitive :type Boolean)))

(fn RemoveArmorBar)

(fn UpdateArmor
  (params (Value :type Integer) (UpdateType :type E_UpdateTypes%20Enum)))

(fn RemoveArmor
  (params (Damage_Value :type Integer)))

(fn UpdateMaxArmor
  (params (Max_Armor :type Integer)))

(fn GetCurrentArmor
  (return 0))

(fn GetCurrentMaxArmor
  (return 0))

(fn AddWeaponBar
  (params (Ammo_ValueColor :type Linear%20Color%20Structure) (MaxAmmo_ValueColor :type Linear%20Color%20Structure) (Frame_Color :type Linear%20Color%20Structure) (ProgressColor :type Linear%20Color%20Structure) (WeaponColor :type Linear%20Color%20Structure) (ProgressImpactColor :type Linear%20Color%20Structure)))

(fn RemoveWeaponBar)

(fn AddorUpdateAmmoIcon
  (params (Icon_Slot :type E_AmmoSlots%20Enum) (Slot_AnimColor :type Linear%20Color%20Structure) (Slot_Icon :type User%20Widget%20Class%20Reference)))

(fn RemoveAmmoIcon
  (params (IconSlot :type E_AmmoSlots%20Enum) (bRemoveAllIcons :type Boolean)))

(fn UpdateWeaponBar
  (params (Weapon_Icon :type Object%20Object%20Reference) (Weapon_Name :type String) (Ammo_Type :type E_AmmoType%20Enum) (Stack_Size :type Integer)))

(fn UpdateAmmo
  (params (Ammo :type Integer) (Update_Type :type E_UpdateTypes%20Enum)))

(fn UpdateMaxAmmo
  (params (MaxAmmo :type Integer) (Update_Type :type E_UpdateTypes%20Enum)))

(fn GetCurrentAmmo
  (return 0))

(fn GetCurrentStackSize
  (return 0))

(fn GetCurrentMaxAmmo
  (return 0))

(fn GetCurrentAmmoType
  (return "NewEnumerator0"))

(fn RemoveAmmo
  (params (Ammo :type Integer)))

(fn RemoveMaxAmmo
  (params (MaxAmmo :type Integer)))

(fn AddorUpdateActionSlot
  (params (E_Slot :type E_ActionSlots%20Enum) (Slot_KeyText :type Text) (Slot_KeyColor :type Linear%20Color%20Structure) (Slot_Icon :type Object%20Object%20Reference) (Slot_IconColor :type Linear%20Color%20Structure) (Slot_FrameColor :type Linear%20Color%20Structure) (Slot_FrameShineColor :type Linear%20Color%20Structure)))

(fn RemoveActionSlot
  (params (ActionSlot :type E_ActionSlots%20Enum)))

(fn RemoveAllActionSlots)

(fn SlotImpact
  (params (Slot :type E_ActionSlots%20Enum)))