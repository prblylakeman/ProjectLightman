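; Actor component that acts as the interface to the WB_ActionHUD shooter HUD, covering health, armor, weapon/ammo and action slot bars.
; InitHUD creates and shows the widget; events forward changes to it.
; Getters read current values back from the widget, which additive health and armor updates build on.
; Forwarding events first run HUD_Validator, which rechecks an invalid widget after short delays, then recreates and redisplays it.
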(event Custom|InitHUD
  (params (OwningPlayer :type Player%20Controller%20Object%20Reference))
  ;[0 0 0] Event Init HUD
  (CallFunction|CreateHUD OwningPlayer)
  (CallFunction|DisplayShooterHUD "NewEnumerator0" 1))

(fn CreateHUD
  (params (OwningPlayer :type Player%20Controller%20Object%20Reference))
  (Utilities|IsValid (Variables|Default|GetWB_ActionHUD)
    (:Is%20Valid
      (return))
    (:Is%20Not%20Valid
      (bind _returnvalue (UserInterface|CreateWidget "/Game/CSHUD_ActionBars/UI/WB_ActionHUD.WB_ActionHUD_C" OwningPlayer))
      (Variables|Default|SetWB_ActionHUD _returnvalue))))

(event EventAddHealthBar
  (params (ProgressBar_Color :type Linear%20Color%20Structure) (Progress_Color :type Linear%20Color%20Structure) (Text_Color :type Linear%20Color%20Structure) (Frame_Color :type Linear%20Color%20Structure) (Damage_Color :type Linear%20Color%20Structure) (Health_Color :type Linear%20Color%20Structure) (Icon :type User%20Widget%20Class%20Reference) (IsMaxHealthSensitive :type Boolean))
  ;[0 0 0] Event Add Health Bar
  (Utilities|HUDValidator)
  (Default|AddHealthBar (Variables|Default|GetWB_ActionHUD) ProgressBar_Color Progress_Color Text_Color Frame_Color Damage_Color Icon IsMaxHealthSensitive)
  (Variables|Damage|SetDamageColor Damage_Color)
  (Variables|Damage|SetHealthColor Health_Color))

(event EventRemoveHealthBar
  ;[0 0 0] Event Remove Health Bar
  (Utilities|HUDValidator)
  (Default|RemoveHealthBar (Variables|Default|GetWB_ActionHUD)))

(event EventUpdateHealth
  (params (Value :type Integer) (UpdateType :type E_UpdateTypes%20Enum :default "NewEnumerator0"))
  ;[0 0 0] Event Update Health
  (Utilities|HUDValidator)
  (switch Utilities|FlowControl|Switch|SwitchonE_UpdateTypes UpdateType
    (:NewEnumerator0
      (Default|UpdateHealth (Variables|Default|GetWB_ActionHUD) Value))
    (:NewEnumerator1
      (bind _healthvalue (CallFunction|GetCurrentHealth))
      (Default|UpdateHealth (Variables|Default|GetWB_ActionHUD) (+ _healthvalue Value)))))

(event EventUpdateMaxHealth
  (params (Max_Health_Value :type Integer))
  ;[0 0 0] Event Update Max Health
  (Utilities|HUDValidator)
  (Default|UpdateMaxHealth (Variables|Default|GetWB_ActionHUD) Max_Health_Value))

(event EventRemoveHealth
  (params (DamageValue :type Integer))
  ;[0 0 0] Event Remove Health
  (Utilities|HUDValidator)
  (Default|RemoveHealth (Variables|Default|GetWB_ActionHUD) DamageValue))

(event EventRemoveAmmoIcon
  (params (IconSlot :type E_AmmoSlots%20Enum :default "NewEnumerator0") (bRemoveAllIcons :type Boolean))
  ;[0 0 0] Event Remove Ammo Icon
  (Utilities|HUDValidator)
  (Default|RemoveAmmoIcon (Variables|Default|GetWB_ActionHUD) IconSlot bRemoveAllIcons))

(event EventUpdateAmmo
  (params (Ammo :type Integer) (Update_Type :type E_UpdateTypes%20Enum :default "NewEnumerator0"))
  ;[0 0 0] Event Update Ammo
  (Utilities|HUDValidator)
  (Default|UpdateAmmo (Variables|Default|GetWB_ActionHUD) Ammo Update_Type))

(event EventUpdateMaxAmmo
  (params (MaxAmmo :type Integer) (Update_Type :type E_UpdateTypes%20Enum :default "NewEnumerator0"))
  ;[0 0 0] Event Update Max Ammo
  (Utilities|HUDValidator)
  (Default|UpdateMaxAmmo (Variables|Default|GetWB_ActionHUD) MaxAmmo Update_Type))

(event EventUpdateWeaponBar
  (params (Weapon_Icon :type Object%20Object%20Reference) (Weapon_Name :type String) (Ammo_Type :type E_AmmoType%20Enum :default "NewEnumerator0") (Stack_Size :type Integer))
  ;[0 0 0] Event Update Weapon Bar
  (Utilities|HUDValidator)
  (Default|UpdateWeaponBar (Variables|Default|GetWB_ActionHUD) Weapon_Icon Weapon_Name Ammo_Type Stack_Size))

(event EventRemoveAmmo
  (params (Ammo :type Integer))
  ;[0 0 0] Event Remove Ammo
  (Utilities|HUDValidator)
  (Default|RemoveAmmo (Variables|Default|GetWB_ActionHUD) Ammo))

(event EventRemoveMaxAmmo
  (params (MaxAmmo :type Integer))
  ;[0 0 0] Event Remove Max Ammo
  (Utilities|HUDValidator)
  (Default|RemoveMaxAmmo (Variables|Default|GetWB_ActionHUD) MaxAmmo))

(event EventAddWeaponBar
  (params (Ammo_ValueColor :type Linear%20Color%20Structure) (MaxAmmo_ValueColor :type Linear%20Color%20Structure) (Frame_Color :type Linear%20Color%20Structure) (ProgressColor :type Linear%20Color%20Structure) (WeaponColor :type Linear%20Color%20Structure) (ProgressImpactColor :type Linear%20Color%20Structure))
  ;[0 0 0] Event Add Weapon Bar
  (Utilities|HUDValidator)
  (Default|AddWeaponBar (Variables|Default|GetWB_ActionHUD) Ammo_ValueColor Frame_Color Ammo_ValueColor MaxAmmo_ValueColor ProgressColor WeaponColor ProgressImpactColor))

(event EventRemoveWeaponBar
  ;[0 0 0] Event Remove Weapon Bar
  (Utilities|HUDValidator)
  (Default|RemoveWeaponBar (Variables|Default|GetWB_ActionHUD)))

(event EventAddorUpdateAmmoIcon
  (params (Icon_Slot :type E_AmmoSlots%20Enum :default "NewEnumerator0") (Slot_AnimColor :type Linear%20Color%20Structure) (Slot_Icon :type User%20Widget%20Class%20Reference))
  ;[0 0 0] Event Add Or Update Ammo Icon
  (Utilities|HUDValidator)
  (Default|AddorUpdateAmmoIcon (Variables|Default|GetWB_ActionHUD) Icon_Slot Slot_AnimColor Slot_Icon))

(event EventSlotImpact
  (params (Slot :type E_ActionSlots%20Enum :default "NewEnumerator0"))
  ;[0 0 0] Event Slot Impact
  (Utilities|HUDValidator)
  (Default|SlotImpact (Variables|Default|GetWB_ActionHUD) Slot))

(event EventAddorUpdateActionSlot
  (params (E_Slot :type E_ActionSlots%20Enum :default "NewEnumerator0") (Slot_KeyText :type Text) (Slot_KeyColor :type Linear%20Color%20Structure) (Slot_Icon :type Object%20Object%20Reference) (Slot_IconColor :type Linear%20Color%20Structure) (Slot_FrameColor :type Linear%20Color%20Structure) (Slot_FrameShineColor :type Linear%20Color%20Structure))
  ;[0 0 0] Event Add Or Update Action Slot
  (Utilities|HUDValidator)
  (Default|AddorUpdateActionSlot (Variables|Default|GetWB_ActionHUD) E_Slot Slot_KeyText Slot_KeyColor Slot_Icon Slot_IconColor Slot_FrameColor Slot_FrameShineColor))

(event EventRemoveActionSlot
  (params (ActionSlot :type E_ActionSlots%20Enum :default "NewEnumerator0"))
  ;[0 0 0] Event Remove Action Slot
  (Utilities|HUDValidator)
  (Default|RemoveActionSlot (Variables|Default|GetWB_ActionHUD) ActionSlot))

(event EventRemoveAllActionSlots
  ;[0 0 0] Event Remove All Action Slots
  (Utilities|HUDValidator)
  (Default|RemoveAllActionSlots (Variables|Default|GetWB_ActionHUD)))

(event EventDisplayShooterHUD
  (params (State :type E_DisplayStates%20Enum :default "NewEnumerator0") (ZOrder :type Integer))
  ;[0 0 0] Event Display Shooter HUD
  (Variables|Default|SetZOrder ZOrder)
  (CallFunction|CreateHUD)
  (|HandleDisplayShooterHUD_2 State))

(event EventAddArmorBar
  (params (ProgressBar_Color :type Linear%20Color%20Structure) (Progress_Color :type Linear%20Color%20Structure) (Text_Color :type Linear%20Color%20Structure) (Frame_Color :type Linear%20Color%20Structure) (Damage_Color :type Linear%20Color%20Structure) (Armor_Color :type Linear%20Color%20Structure) (Armor_Icon :type User%20Widget%20Class%20Reference) (MaxArmorSensitive :type Boolean))
  ;[0 0 0] Event Add Armor Bar
  (Utilities|HUDValidator)
  (Default|AddArmorBar (Variables|Default|GetWB_ActionHUD) ProgressBar_Color Progress_Color Text_Color Frame_Color Damage_Color Armor_Icon MaxArmorSensitive)
  (Variables|Armor|SetArmorColor Armor_Color)
  (Variables|Armor|SetArmorDamageColor Damage_Color))

(event EventRemoveArmorBar
  ;[0 0 0] Event Remove Armor Bar
  (Utilities|HUDValidator)
  (Default|RemoveArmorBar (Variables|Default|GetWB_ActionHUD)))

(event EventUpdateArmor
  (params (Value :type Integer) (UpdateType :type E_UpdateTypes%20Enum :default "NewEnumerator0"))
  ;[0 0 0] Event Update Armor
  (Utilities|HUDValidator)
  (switch Utilities|FlowControl|Switch|SwitchonE_UpdateTypes UpdateType
    (:NewEnumerator0
      (Default|UpdateArmor (Variables|Default|GetWB_ActionHUD) Value))
    (:NewEnumerator1
      (bind _armorvalue (CallFunction|GetCurrentArmor))
      (Default|UpdateArmor (Variables|Default|GetWB_ActionHUD) (+ _armorvalue Value)))))

(event EventRemoveArmor
  (params (Damage_Value :type Integer))
  ;[0 0 0] Event Remove Armor
  (Utilities|HUDValidator)
  (Default|RemoveArmor (Variables|Default|GetWB_ActionHUD) Damage_Value))

(event EventUpdateMaxArmor
  (params (Max_Armor :type Integer))
  ;[0 0 0] Event Update Max Armor
  (Utilities|HUDValidator)
  (Default|UpdateMaxArmor (Variables|Default|GetWB_ActionHUD) Max_Armor))

(fn GetCurrentAmmo
  (bind _wb_actionhud (Variables|Default|GetWB_ActionHUD))
  (Utilities|IsValid _wb_actionhud
    (:Is%20Valid
      (return (Default|GetCurrentAmmo _wb_actionhud)))
    (:Is%20Not%20Valid
      (return 0))))

(fn GetCurrentAmmoType
  (bind _wb_actionhud (Variables|Default|GetWB_ActionHUD))
  (Utilities|IsValid _wb_actionhud
    (:Is%20Valid
      (return (Default|GetCurrentAmmoType _wb_actionhud)))
    (:Is%20Not%20Valid
      (return "NewEnumerator0"))))

(fn GetCurrentArmor
  (bind _wb_actionhud (Variables|Default|GetWB_ActionHUD))
  (Utilities|IsValid _wb_actionhud
    (:Is%20Valid
      (bind _currentarmor (Default|GetCurrentArmor _wb_actionhud))
      (return _currentarmor))
    (:Is%20Not%20Valid
      (return 0))))

(fn GetCurrentHealth
  (bind _wb_actionhud (Variables|Default|GetWB_ActionHUD))
  (Utilities|IsValid _wb_actionhud
    (:Is%20Valid
      (bind _currenthealth (Default|GetCurrentHealth _wb_actionhud))
      (return _currenthealth))
    (:Is%20Not%20Valid
      (return 0))))

(fn GetCurrentMaxAmmo
  (bind _wb_actionhud (Variables|Default|GetWB_ActionHUD))
  (Utilities|IsValid _wb_actionhud
    (:Is%20Valid
      (return (Default|GetCurrentMaxAmmo _wb_actionhud)))
    (:Is%20Not%20Valid
      (return 0))))

(fn GetCurrentMaxArmor
  (bind _wb_actionhud (Variables|Default|GetWB_ActionHUD))
  (Utilities|IsValid _wb_actionhud
    (:Is%20Valid
      (bind _currentmaxarmor (Default|GetCurrentMaxArmor _wb_actionhud))
      (return _currentmaxarmor))
    (:Is%20Not%20Valid
      (return 0))))

(fn GetCurrentMaxHealth
  (bind _wb_actionhud (Variables|Default|GetWB_ActionHUD))
  (Utilities|IsValid _wb_actionhud
    (:Is%20Valid
      (bind _currentmaxhealth (Default|GetCurrentMaxHealth _wb_actionhud))
      (return _currentmaxhealth))
    (:Is%20Not%20Valid
      (return 0))))

(fn GetCurrentStackSize
  (bind _wb_actionhud (Variables|Default|GetWB_ActionHUD))
  (Utilities|IsValid _wb_actionhud
    (:Is%20Valid
      (return (Default|GetCurrentStackSize _wb_actionhud)))
    (:Is%20Not%20Valid
      (return 0))))