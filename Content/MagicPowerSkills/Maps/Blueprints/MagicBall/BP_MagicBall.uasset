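; Magic ball actor for the magic power skills, a glowing sphere with an effect trail that plays timed visual sequences and then destroys itself.
; Reusable timeline events, rate-scaled to a duration, drive movement, scale, and the glow and opacity of a dynamic material on the sphere.
; Preset events (ScaleAndUp, Attraction, Direct, Up) chain these with delays to charge, glow and fade, with some detaching and launching the ball.
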(fn ConstructionScript)

(fn TrailActivate
  (params (Active :type Boolean))
  (Components|Activation|SetActive (Variables|Default|GetEffectTrail) Active false))

(event Custom|MoveActor
  (params (Forward :type Boolean) (ForwardVector :type Vector) (Disatnce :type Float%20%28double-precision%29) (Location :type Vector) (Time :type Float%20%28double-precision%29))
  (Variables|Movement|SetStartLoc (Transformation|GetActorLocation))
  (if Forward
    (Variables|Movement|SetEndLoc (+ (Variables|Movement|GetStartLoc) (* ForwardVector Disatnce)))
    (else
      (Variables|Movement|SetEndLoc Location)))
  (Components|Timeline|SetPlayRate (Variables|Default|GetTM_Movement) (/ 1.0 Time))
  (bind _alpha (Timeline|TM_Movement PlayFromStart)
    (:Update
      (Transformation|SetActorLocation (Math|Vector|Lerp(Vector) (Variables|Movement|GetStartLoc) (Variables|Movement|GetEndLoc) _alpha) false false))))

(event Custom|SetGlow
  (params (Glow :type Boolean) (Time :type Float%20%28double-precision%29))
  (Components|Timeline|SetPlayRate (Variables|Default|GetTM_Glow) (/ 1.0 Time))
  (if Glow
    (bind _alpha (Timeline|TM_Glow Play)
      (:Update
        (bind _output_get (Variables|Glow|SetGlowCurrent (Math|Float|Lerp 3.6 -1.0 _alpha)))
        (Rendering|Material|SetScalarParameterValue (Variables|Components|GetMaterial) "ExponentIn" _output_get :!class /Script/Engine.MaterialInstanceDynamic)))
    (else
      (Timeline|TM_Glow Reverse))))

(event Custom|SetScale
  (params (Time :type Float%20%28double-precision%29) (Scale :type Vector))
  (Components|Timeline|SetPlayRate (Variables|Default|GetTM_Scale) (/ 1.0 Time))
  (Variables|Scale|SetScaleTarget Scale)
  (Variables|Scale|SetScaleCurrent (Transformation|GetActorScale3D))
  (bind _alpha (Timeline|TM_Scale PlayFromStart)
    (:Update
      (Transformation|SetActorScale3D (Math|Vector|Lerp(Vector) (Variables|Scale|GetScaleCurrent) (Variables|Scale|GetScaleTarget) _alpha)))))

(event EventBeginPlay
  (bind _returnvalue (Rendering|Material|CreateDynamicMaterialInstance (Variables|Default|GetSphere) 0 "/Game/MagicPowerSkills/Demo/Effects/Materials/MI_MagicShield.MI_MagicShield" "None" :!class /Script/Engine.PrimitiveComponent))
  (Variables|Components|SetMaterial _returnvalue))

(event Custom|SetOpacity
  (params (Time :type Float%20%28double-precision%29) (Opacity :type Float%20%28double-precision%29))
  (Components|Timeline|SetPlayRate (Variables|Default|GetTM_Opacity) (/ 1.0 Time))
  (Variables|Default|SetTargetOpacity Opacity)
  (bind _returnvalue (Rendering|Material|GetScalarParameterValue (Variables|Components|GetMaterial) "Opacity" :!class /Script/Engine.MaterialInstanceDynamic))
  (Variables|Default|SetCurrentOpacity _returnvalue)
  (bind _alpha (Timeline|TM_Opacity PlayFromStart)
    (:Update
      (Rendering|Material|SetScalarParameterValue (Variables|Components|GetMaterial) "Opacity" (Math|Float|Lerp (Variables|Default|GetCurrentOpacity) (Variables|Default|GetTargetOpacity) _alpha) :!class /Script/Engine.MaterialInstanceDynamic))))

(event Custom|ScaleAndUp
  (bind _returnvalue (Transformation|GetActorLocation))
  (CallFunction|SetScale 1.1 "1.500000,1.500000,1.500000")
  (CallFunction|SetGlow true 1.05)
  (Utilities|FlowControl|Delay 1.1)
  (CallFunction|MoveActor false "0, 0, 0" 0.0 (Math|Vector|MakeVector (.x _returnvalue) (.y _returnvalue) (+ (.z _returnvalue) 6e+02)) 0.5)
  (CallFunction|SetOpacity 0.5 0.0)
  (CallFunction|SetGlow false 0.5)
  (Utilities|FlowControl|Delay 4.0)
  (Actor|DestroyActor))

(event Custom|Attraction
  (params (Time :type Float%20%28double-precision%29))
  (CallFunction|SetOpacity 0.1 0.0)
  (CallFunction|SetScale Time "1.000000,1.000000,1.000000")
  (CallFunction|SetOpacity Time 0.7)
  (CallFunction|SetGlow true (+ Time 0.1))
  (Utilities|FlowControl|Delay (+ Time 0.2))
  (CallFunction|SetGlow false 0.4)
  (CallFunction|SetOpacity 0.4 0.0)
  (CallFunction|TrailActivate false)
  (Utilities|FlowControl|Delay 3.0)
  (Actor|DestroyActor))

(event Custom|Direct
  (params (Time :type Float%20%28double-precision%29) (ForwardVector :type Vector))
  (CallFunction|SetOpacity 0.01 0.0)
  (CallFunction|SetScale Time "1.500000,1.500000,1.500000")
  (CallFunction|SetOpacity Time 0.7)
  (CallFunction|SetGlow true Time)
  (Utilities|FlowControl|Delay Time)
  (Transformation|DetachFromActor "KeepWorld" "KeepWorld" "KeepWorld")
  (CallFunction|MoveActor true ForwardVector 8e+02 "0, 0, 0" 1.0)
  (CallFunction|SetGlow false 0.5)
  (CallFunction|SetOpacity 0.5 0.0)
  (Utilities|FlowControl|Delay 3.0)
  (CallFunction|TrailActivate false)
  (Utilities|FlowControl|Delay 3.0)
  (Actor|DestroyActor))

(event Custom|Up
  (params (Time :type Float%20%28double-precision%29) (ForwardVector :type Vector))
  (CallFunction|SetOpacity 0.01 0.0)
  (CallFunction|SetScale Time "1.500000,1.500000,1.500000")
  (CallFunction|SetOpacity Time 0.7)
  (CallFunction|SetGlow true Time)
  (Utilities|FlowControl|Delay Time)
  (Transformation|DetachFromActor "KeepWorld" "KeepWorld" "KeepWorld")
  (CallFunction|MoveActor false ForwardVector 8e+02 (+ (Transformation|GetActorLocation) ForwardVector) 1.0)
  (CallFunction|SetGlow false 0.5)
  (CallFunction|SetOpacity 0.5 0.0)
  (Utilities|FlowControl|Delay 3.0)
  (CallFunction|TrailActivate false)
  (Utilities|FlowControl|Delay 3.0)
  (Actor|DestroyActor))