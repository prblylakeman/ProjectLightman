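; Blueprint function library that looks up reward card data in the DT_Rewards data table.
; MF_GetCardInfoByID scans the rows for the first matching CardID and returns it with a found flag, printing a message on a miss.
; MF_GetRewardCardForLevel collects every row whose RewardForLevel matches the given level completion and reports whether any were found.
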(fn MFGetCardInfobyID
  (params (CardID :type Integer))
  (bind _outrownames (DataTable|GetDataTableRowNames "/Game/RewardCards/DataTables/DT_Rewards.DT_Rewards"))
  (bind _array_element (Utilities|Array|ForEachLoopwithBreak _outrownames :!label _label)
    (:LoopBody
      (bind _returnvalue (Utilities|GetDataTableRow "/Game/RewardCards/DataTables/DT_Rewards.DT_Rewards" _array_element)
        (:then
          (if (== (.CardID (Utilities|Struct|BreakS_CardInfo _returnvalue)) CardID)
            (LocalVariables|SetCardInfoByID _returnvalue)
            (LocalVariables|SetFound true)
            (goto _label Break)))))
    (:Completed
      (if (LocalVariables|GetFound)
        (return (LocalVariables|GetCardInfoByID) (LocalVariables|GetFound))
        (else
          (Development|PrintString 0 "Card Info By Card ID not found")
          (return "" false))))))

(fn MFGetRewardCardforLevel
  (params (LevelCompletion :type Integer))
  (bind _rewardcardsforcertainlevel (LocalVariables|GetRewardCardsForCertainLevel))
  (bind _outrownames (DataTable|GetDataTableRowNames "/Game/RewardCards/DataTables/DT_Rewards.DT_Rewards"))
  (for _array_element _outrownames
    (bind _returnvalue (Utilities|GetDataTableRow "/Game/RewardCards/DataTables/DT_Rewards.DT_Rewards" _array_element)
      (:then
        (if (== (.RewardForLevel (Utilities|Struct|BreakS_CardInfo _returnvalue)) LevelCompletion)
          (Utilities|Array|Add (LocalVariables|GetRewardCardsForCertainLevel) _returnvalue)))))
  (return _rewardcardsforcertainlevel (> (Utilities|Array|Length _rewardcardsforcertainlevel) 0)))