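; AC_RandomCard is a helper that picks one reward card from a level's list using weighted random selection.
; GetRandomRewardCard totals every card's RewardChance through GetSum and stores it as OverallPercents.
; ChooseReward rolls a float up to that total and walks the list, subtracting each chance until the roll lands on a card.
; Chances act as relative weights, so they need not add up to 100.
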(fn GetSum
  (params (Rewards :type Array%20of%20S%20Card%20Info%20Structures))
  (for _array_element Rewards
    (LocalVariables|SetSum (+ (Utilities|Struct|BreakS_CardInfo _array_element) (LocalVariables|GetSum))))
  (return (LocalVariables|GetSum)))

(fn ChooseReward
  (params (Reward :type Array%20of%20S%20Card%20Info%20Structures))
  (LocalVariables|SetRandomVal (Math|Random|RandomFloatinRange 0.0 (Variables|Default|GetOverallPercents)))
  (for _array_element Reward
    (if (< (LocalVariables|GetRandomVal) (.RewardChance (Utilities|Struct|BreakS_CardInfo _array_element)))
      (return _array_element)
      (else
        (LocalVariables|SetRandomVal (- (LocalVariables|GetRandomVal) (.RewardChance (Utilities|Struct|BreakS_CardInfo _array_element))))))))

(fn GetRandomRewardCard
  (params (LevelRewardCards :type Array%20of%20S%20Card%20Info%20Structures))
  (Variables|Default|SetOverallPercents (CallFunction|GetSum LevelRewardCards))
  (bind _cardinfo (CallFunction|ChooseReward LevelRewardCards))
  (return _cardinfo))