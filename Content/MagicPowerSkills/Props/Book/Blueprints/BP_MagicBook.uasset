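; BP_MagicBook is a magic book prop that opens and closes with animated, glowing text, expecting a BP_CharWithMagicItem owner.
; OpenBook sets a use flag on AnimBP_Book and controls the book mesh's visibility.
; A shared GlowEffect timeline drives the dynamic text material, fading in opacity and emissive after a delay on open, or using a separate opacity curve on close.
; Closing hides the mesh after a retriggerable delay, unless it is in use again.
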(event Custom|OpenBook
  (params (Open? :type Boolean))
  (if Open?
    (Rendering|SetVisibility (Variables|Default|GetBook) true false)
    (Rendering|Material|SetScalarParameterValue (Variables|Effects|GetTextMaterial) "Opacity" 0.0 :!class /Script/Engine.MaterialInstanceDynamic)
    (Rendering|Material|SetScalarParameterValue (Variables|Effects|GetTextMaterial) "EmStrength" 0.0 :!class /Script/Engine.MaterialInstanceDynamic)
    (Variables|/Game/MagicPowerSkills/Props/Book/Blueprints/AnimBP_Book.AnimBP_Book_C|SetIsUseBook (Variables|Components|GetAnimBP) true)
    (Utilities|FlowControl|RetriggerableDelay 1.2)
    (bind (_direction _alphaemmisive _opacityalpha _unequipalpha) (Timeline|GlowEffect PlayFromStart)
      (:Update
        (if Open?
          (Rendering|Material|SetScalarParameterValue (Variables|Effects|GetTextMaterial) "EmStrength" _alphaemmisive :!class /Script/Engine.MaterialInstanceDynamic)
          (Rendering|Material|SetScalarParameterValue (Variables|Effects|GetTextMaterial) "Opacity" _opacityalpha :!class /Script/Engine.MaterialInstanceDynamic)
          (else
            (Rendering|Material|SetScalarParameterValue (Variables|Effects|GetTextMaterial) "Opacity" _unequipalpha :!class /Script/Engine.MaterialInstanceDynamic)))))
    (else
      (Variables|/Game/MagicPowerSkills/Props/Book/Blueprints/AnimBP_Book.AnimBP_Book_C|SetIsUseBook (Variables|Components|GetAnimBP) false)
      (Utilities|FlowControl|Sequence
        (:then_0
          (Timeline|GlowEffect PlayFromStart))
        (:then_1
          (Utilities|FlowControl|RetriggerableDelay 0.8)
          (if (not (Variables|/Game/MagicPowerSkills/Props/Book/Blueprints/AnimBP_Book.AnimBP_Book_C|GetIsUseBook (Variables|Components|GetAnimBP)))
            (Rendering|SetVisibility (Variables|Default|GetBook) false false)))))))

(event EventBeginPlay
  (bind _returnvalue (Rendering|Material|CreateDynamicMaterialInstance (Variables|Default|GetBook) 2 "/Game/MagicPowerSkills/Props/Book/Materials/MI_BookText.MI_BookText" "Text" :!class /Script/Engine.PrimitiveComponent))
  (Variables|Effects|SetTextMaterial _returnvalue)
  (bind _asanim_bp_book (Utilities|Casting|CastToAnimBP_Book (Components|SkeletalMesh|GetAnimInstance (Variables|Default|GetBook))))
  (Variables|Components|SetAnimBP _asanim_bp_book)
  (bind _asbp_char_with_magic_item (Utilities|Casting|CastToBP_CharWithMagicItem (Components|GetOwner)))
  (Variables|Components|SetCharacterOwner _asbp_char_with_magic_item))

(fn ConstructionScript)